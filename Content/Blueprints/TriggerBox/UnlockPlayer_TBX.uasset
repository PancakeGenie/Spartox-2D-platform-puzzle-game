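; Trigger box that unlocks pawn switching for the player when its overlap event fires.
; On overlap, it replaces all widgets with an UnlockPawn notice, then removes all widgets after a short delay.
; In the same sequence, without waiting for the delay, it enables switching on the player's BluePawn_BP.
; It also spawns a key item at a hardcoded location and sets MultipleOverlaps to false.
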(event EventOnTriggerOverlap
  (Utilities|FlowControl|Sequence
    (:then_0
      ;[1 1 1] Create UnlockPawn widget and remove previous widgets
      (Viewport|RemoveAllWidgets)
      (bind _returnvalue (UserInterface|CreateWidget "/Game/Blueprints/Widgets/UnlockPawn_WBP.UnlockPawn_WBP_C"))
      (UserInterface|Viewport|AddtoViewport _returnvalue 0)
      (Utilities|FlowControl|Delay 2.0)
      (Viewport|RemoveAllWidgets))
    (:then_1
      ;[1 1 1] Allow player to jump
      (bind _asblue_pawn_bp (Utilities|Casting|CastToBluePawn_BP (Game|Player|GetPlayerPawn 0)))
      (Class|BasePawn|SetCanPlayerSwitch _asblue_pawn_bp true))
    (:then_2
      (Game|SpawnActorfromClass "/Game/Blueprints/Actors/Collectables/KeyItem_BP.KeyItem_BP_C" (Math|Transform|MakeTransform "-1418.000000, 0,-230.000000" "0, 0, 0" "1,1,1") "Undefined" 0 0)
      (Variables|Default|SetbMultipleOverlaps false))))

(fn ConstructionScript)